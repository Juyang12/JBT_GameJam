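; BP_Box is a box the player can push, with PushStart and PushEnd toggling the pushing state.
; While the BP_BaseActor player moves during a push, Tick interpolates the Cube along the player's forward vector by horizontal input and Speed, without sweep.
; An IsFalling check ends the push and restores walk speed, though its velocity test is unwired.
; A FaceToCharacter yaw helper goes uncalled here.
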(event EventBeginPlay
  (|CallParentFunction)
  (bind _asbp_base_actor (Utilities|Casting|CastToBP_BaseActor (Game|Player|GetPlayerPawn 0)))
  (Variables|Default|SetAs%20BP%20Base%20Actor _asbp_base_actor))

(event Collision|EventActorBeginOverlap
  (params (OtherActor :type Actor%20Object%20Reference))
  (|CallParentFunction OtherActor) ; 此节点被禁用，将不会被调用。\n从引脚连出引线来编译功能。
)

(event EventTick
  (params (DeltaSeconds :type Float%20%28single-precision%29))
  (bind _as_bp_base_actor (Variables|Default|GetAs%20BP%20Base%20Actor))
  (|CallParentFunction DeltaSeconds)
  (if (and (Variables|Default|GetIsPushing) (Utilities|Operators|NotEqual(!=) :A (Transformation|GetVelocity (Variables|Default|GetAs%20BP%20Base%20Actor))))
    (Utilities|FlowControl|Sequence
      (:then_0
        (if (AI|Components|NavMovement|IsFalling)
          (CallFunction|PushEnd)
          (Variables|/Game/Blueprint/BP_BaseActor.BP_BaseActor_C|SetIsPushing _as_bp_base_actor false)
          (Variables|/Script/Engine.CharacterMovementComponent|SetMaxWalkSpeed (Variables|/Script/Engine.Character|GetCharacterMovement _as_bp_base_actor) (Variables|/Game/Blueprint/BP_BaseActor.BP_BaseActor_C|GetwalkSpeed _as_bp_base_actor))))
      (:then_1
        (Utilities|Move (* (.x (Variables|/Game/Blueprint/BP_BaseActor.BP_BaseActor_C|GetInput%20Vector (Variables|Default|GetAs%20BP%20Base%20Actor))) (Variables|Default|Getspeed)))))))

(event EventPushStart
  (Development|PrintString "Push")
  (Variables|Default|SetIsPushing true))

(event EventPushEnd
  (Variables|Default|SetIsPushing false))

(fn ConstructionScript
  (|CallParentFunction))