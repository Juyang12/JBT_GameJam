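; Character Blueprint that can push BP_Box actors, with movement relative to its own facing and orient-to-movement disabled when moving backward.
; IA_StickBox toggles pushing: it grabs an overlapping box via BPI_Push and slows walking, or releases the first interface actor found and restores speed.
; The IsFaceToBox dot-product check is left unwired, and the line trace only feeds debug output.
; Also includes a key-1 HUD hook and a location getter for being seen.
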(event Input|EnhancedActionEvents|EnhancedInputActionIA_StickBox
  (params (ActionValue :type Boolean) (ElapsedSeconds :type Float%20%28double-precision%29) (TriggeredSeconds :type Float%20%28double-precision%29) (InputAction :type Input%20Action%20Object%20Reference :default "/Game/Input/IA_StickBox.IA_StickBox"))
  (bind _self self)
  (bind _returnvalue (Transformation|GetActorLocation _self))
  (:Started
    (bind (_outhit _returnvalue_2) (Collision|LineTraceByChannel _returnvalue (+ _returnvalue (* (Transformation|GetActorForwardVector _self) 2e+02)) "TraceTypeQuery3" false 0 "ForDuration"))
    (Development|PrintString (Utilities|String|ToString(Boolean) _returnvalue_2))
    (if (Variables|Default|GetIsPushing)
      (Variables|Default|SetIsPushing false)
      (bind _outactors (Actor|GetAllActorswithInterface "/Game/Blueprint/Interface/BPI_Push.BPI_Push_C"))
      (bind _array_element (Utilities|Array|ForEachLoopwithBreak _outactors :!label _label)
        (:LoopBody
          (Class|BPIPush|PushEnd(Message) _array_element)
          (Variables|/Script/Engine.CharacterMovementComponent|SetMaxWalkSpeed (Variables|Character|GetCharacterMovement) 6e+02)
          (goto _label Break)))
      (else
        (bind _array_element_2 (Utilities|Array|ForEachLoopwithBreak (Collision|GetOverlappingActors "/Game/Blueprint/BP_Box.BP_Box_C" :!class /Script/Engine.Actor) :!label _label_2)
          (:LoopBody
            (Variables|Default|Setbox _array_element_2)
            (if (and (|IsFaceToBox) (Utilities|DoesObjectImplementInterface _array_element_2 "/Game/Blueprint/Interface/BPI_Push.BPI_Push_C"))
              (Variables|/Script/Engine.CharacterMovementComponent|SetMaxWalkSpeed (Variables|Character|GetCharacterMovement) 98.0)
              (Class|BPIPush|PushStart(Message) (Variables|Default|Getbox))
              (Variables|Default|SetIsPushing true)
              (goto _label_2 Break)
              (else
                (Variables|Default|SetIsPushing false)))))))))

(event EventBeginPlay)

(event Collision|EventActorBeginOverlap
  (params (OtherActor :type Actor%20Object%20Reference)))

(event EventTick
  (params (DeltaSeconds :type Float%20%28single-precision%29)))

(event Input|KeyboardEvents|1
  (params (Key :type Key%20Structure :default "None"))
  (:Pressed
    (Utilities|String|LogString "Hello")
    (bind _asbp_in_game_hud (Utilities|Casting|CastToBP_InGameHUD (HUD|GetHUD (Game|GetPlayerController 0)))
      (:then
        (Default|FUNCShowHUD _asbp_in_game_hud))
      (:CastFailed
        (Game|QuitGame 0 "Quit" false)))))

(fn ConstructionScript)

(event EventMove
  (params (inputVector :type Input%20Action%20Value%20Structure%20%28by%20ref%29))
  (bind (_x _y) (Class|EnhancedInputLibrary|BreakInputActionValue inputVector))
  (if (< _x 0.0)
    (Variables|/Script/Engine.CharacterMovementComponent|SetbOrientRotationToMovement (Variables|Character|GetCharacterMovement) false)
    (else
      (Variables|/Script/Engine.CharacterMovementComponent|SetbOrientRotationToMovement (Variables|Character|GetCharacterMovement) true)))
  (Pawn|Input|AddMovementInput (Math|Vector|Normalize (+ (* (Math|Vector|Normalize (Transformation|GetActorForwardVector) 0.001) _x) (* (Math|Vector|Normalize (Transformation|GetActorRightVector) 0.001) _y)) 0.001) 1.0 false))

(fn FUNConBeenSeen
  (return (Transformation|GetActorLocation)))