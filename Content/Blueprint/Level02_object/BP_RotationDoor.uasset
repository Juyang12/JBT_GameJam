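; BP_RotationDoor is a door in the Level02 object set that rotates its Cube when signalled through the EDRorder binding made at BeginPlay.
; DOROTATION branches on IsRotation, either playing RotationTimeLine from the start or reversing a second Timeline from its end.
; Each timeline's track sets the Cube's relative pitch through the Undo/Do 90 Rotation functions.
; IsRotation flips on every timeline update, rather than on completion.
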(event Custom|DOROTATION
  (if (Variables|Default|GetisRotation)
    (bind _newtrack_0 (Timeline|RotationTimeLine PlayFromStart)
      (:Update
        (CallFunction|FUNCUndo90Rotation _newtrack_0)))
    (else
      (bind _newtrack_0_2 (Timeline|Timeline ReverseFromEnd)
        (:Update
          (CallFunction|FUNCDo90Rotation _newtrack_0_2)))))
  (Variables|Default|SetisRotation (not (Variables|Default|GetisRotation))))

(event EventBeginPlay
  (|CallParentFunction)
  (EventDispatchers|BindEventtoEDRorder (delegate Custom|DOROTATION)))

(event Collision|EventActorBeginOverlap
  (params (OtherActor :type Actor%20Object%20Reference))
  (|CallParentFunction OtherActor) ; This node is disabled and will not be called.\nDrag off pins to build functionality.
)

(event EventTick
  (params (DeltaSeconds :type Float%20%28single-precision%29))
  (|CallParentFunction DeltaSeconds) ; This node is disabled and will not be called.\nDrag off pins to build functionality.
)

(fn ConstructionScript
  (|CallParentFunction))

(fn FUNCDo90Rotation
  (params (val :type Float%20%28double-precision%29))
  (Transformation|SetRelativeRotation (Variables|Default|GetCube) (Math|Rotator|MakeRotator 0.0 val 0.0) false false))

(fn FUNCUndo90Rotation
  (params (val :type Float%20%28double-precision%29))
  (Transformation|SetRelativeRotation (Variables|Default|GetCube) (Math|Rotator|MakeRotator 0.0 val 0.0) false false))